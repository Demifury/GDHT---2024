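; Player controller for a car game that handles per-player setup, menu and ready input, and camera toggling.
; ConnecttoGame uses the player index to pick a team color, view a matching CineCamera and add the menu input context.
; Ready input swaps the menu mapping context for the ready one once.
; Camera toggle flip-flops between the pawn view and that CineCamera, switching the back spring arm's rotation inheritance.
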(event `self.ReceiveBeginPlay`
  (`WidgetBlueprintLibrary.SetInputMode_GameAndUIEx` self null))

(event `EnhancedInput|/Game/Blueprints/Input/Actions/IA_NextCar`
  (params (ActionValue :type Boolean) (ElapsedSeconds :type "Float (double-precision)") (TriggeredSeconds :type "Float (double-precision)") (InputAction :type "InputAction Object Reference" :default "/Game/Blueprints/Input/Actions/IA_NextCar.IA_NextCar")))

(event `EnhancedInput|/Game/Blueprints/Input/Actions/IA_PreviuosCar`
  (params (ActionValue :type Boolean) (ElapsedSeconds :type "Float (double-precision)") (TriggeredSeconds :type "Float (double-precision)") (InputAction :type "InputAction Object Reference" :default "/Game/Blueprints/Input/Actions/IA_PreviuosCar.IA_PreviuosCar")))

(event `EnhancedInput|/Game/Blueprints/Input/Actions/IA_Ready`
  (params (ActionValue :type Boolean) (ElapsedSeconds :type "Float (double-precision)") (TriggeredSeconds :type "Float (double-precision)") (InputAction :type "InputAction Object Reference" :default "/Game/Blueprints/Input/Actions/IA_Ready.IA_Ready"))
  (bind _returnvalue (subsystem `EnhancedInputLocalPlayerSubsystem`))
  (:`Started`
    (`/Engine/EditorBlueprintResources/StandardMacros.DoOnce` false
      (:`Completed`
        (set `self.bReady?` false)
        (`EnhancedInputSubsystemInterface.RemoveMappingContext` _returnvalue "/Game/Blueprints/Input/MappingContexts/IMC_Menu.IMC_Menu" (struct))
        (`EnhancedInputSubsystemInterface.AddMappingContext` _returnvalue "/Game/Blueprints/Input/MappingContexts/IMC_Ready.IMC_Ready" 0 (struct))))))

(event `EnhancedInput|/Game/Blueprints/Input/Actions/IA_ToggleCamera`
  (params (ActionValue :type Boolean) (ElapsedSeconds :type "Float (double-precision)") (TriggeredSeconds :type "Float (double-precision)") (InputAction :type "InputAction Object Reference" :default "/Game/Blueprints/Input/Actions/IA_ToggleCamera.IA_ToggleCamera"))
  (bind _returnvalue (`self.K2_GetPawn`))
  (:`Started`
    (if (not (`self.bSwitchCamera`))
      (bind _asvehicle_adv_pawn (cast `/Game/Blueprints/Vehicles/Default/VehicleAdvPawn` _returnvalue))
      (`/Engine/EditorBlueprintResources/StandardMacros.FlipFlop`
        (:`A`
          (bind _backspringarm (`/Game/Blueprints/Vehicles/Default/VehicleAdvPawn.BackSpringArm` _asvehicle_adv_pawn))
          (set `SpringArmComponent.bInheritRoll` true _backspringarm)
          (set `SpringArmComponent.bInheritPitch` true _backspringarm)
          (set `SpringArmComponent.bInheritYaw` true _backspringarm)
          (`self.SetViewTargetWithBlend` self _returnvalue 0.0 "VTBlend_Linear" 0.0 false))
        (:`B`
          (set `SpringArmComponent.bInheritRoll` false _backspringarm)
          (set `SpringArmComponent.bInheritPitch` false _backspringarm)
          (set `SpringArmComponent.bInheritYaw` false _backspringarm)
          (bind _outactors (`GameplayStatics.GetAllActorsOfClass` "/Script/CinematicCamera.CineCameraActor"))
          (`self.SetViewTargetWithBlend` self (`|GetArrayItem` _outactors (`self.iPlayerIndex`)) 0.0 "VTBlend_Linear" 0.0 false)
          (`SceneComponent.K2_SetRelativeRotation` _backspringarm (struct :`Pitch` 90.0) false false))))))

(event `/Game/Blueprints/BPI_StartGame.ConnectToGame`
  (params (PlayerIndex :type Integer))
  (bind _output_get (set `self.iPlayerIndex` PlayerIndex))
  (`self.SetCarColor` _output_get)
  (bind _outactors (`GameplayStatics.GetAllActorsOfClass` "/Script/CinematicCamera.CineCameraActor"))
  (bind _output (`|GetArrayItem` _outactors (`self.iPlayerIndex`)))
  (`self.SetViewTargetWithBlend` _output)
  (`self.K2_AttachToComponent` _output null "None" "KeepWorld" "KeepWorld" "KeepWorld" true)
  (`EnhancedInputSubsystemInterface.AddMappingContext` (subsystem `EnhancedInputLocalPlayerSubsystem`) "/Game/Blueprints/Input/MappingContexts/IMC_Menu.IMC_Menu" 0 (struct)))

(event `/Game/Blueprints/BPI_StartGame.StartGame`
  (`EnhancedInputSubsystemInterface.AddMappingContext` (subsystem `EnhancedInputLocalPlayerSubsystem`) "/Game/Blueprints/Input/MappingContexts/IMC_Menu.IMC_Menu" 0 (struct))
  (`WidgetBlueprintLibrary.SetInputMode_GameOnly` self)
  (set `self.bShowMouseCursor` false))

(fn `UserConstructionScript`)